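; BP_NPC is the Gatekeeper quest NPC, who talks to the player about a lost statue and completes the quest once it is found.
; A trigger box, sized in the construction script, enables input while the player overlaps it, so the Action key opens a reused W_NPC1 dialogue widget in UI-only mode.
; Later talks swap the text, and if BPRefSmallStatue reports FoundSmallStatue, show thanks and set QuestComplete on ThirdPersonCharacter.
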(event OnComponentBeginOverlap(TriggerZone)
  (params (OverlappedComponent :type Primitive%20Component%20Object%20Reference) (OtherActor :type Actor%20Object%20Reference) (OtherComp :type Primitive%20Component%20Object%20Reference) (OtherBodyIndex :type Integer) (bFromSweep :type Boolean) (SweepResult :type Hit%20Result%20Structure%20%28by%20ref%29))
  ;[1 1 1] GateKeeper Triggerzone
  (if (== OtherActor (Game|GetPlayerCharacter 0))
    (Input|EnableInput (Game|GetPlayerController 0))))

(event OnComponentEndOverlap(TriggerZone)
  (params (OverlappedComponent :type Primitive%20Component%20Object%20Reference) (OtherActor :type Actor%20Object%20Reference) (OtherComp :type Primitive%20Component%20Object%20Reference) (OtherBodyIndex :type Integer))
  ;[1 1 1] GateKeeper Triggerzone
  (if (== OtherActor (Game|GetPlayerCharacter 0))
    (Input|DisableInput (Game|GetPlayerController 0))))

(event Input|ActionEvents|InputActionAction
  (params (Key :type Key%20Structure :default "AnyKey"))
  (bind _returnvalue (Game|GetPlayerController 0))
  ;[1 1 1] Talking to the GateKeeper
  (:Pressed
    (Utilities|IsValid (Variables|Default|GetW_NPC1_ref)
      (:Is%20Valid
        _)
      (:Is%20Not%20Valid
        (bind _returnvalue_2 (UserInterface|CreateWidget "/Game/MyContent/Widgets/W_NPC1.W_NPC1_C" _returnvalue))
        (bind _output_get (Variables|Default|SetW_NPC1_ref _returnvalue_2))))
    (UserInterface|Viewport|AddtoViewport _output_get 0)
    (Input|SetInputModeUIOnly _returnvalue _output_get "DoNotLock")
    (if (Variables|Default|GetbFirstTalkEnded)
      (Variables|/Game/MyContent/Widgets/W_NPC1.W_NPC1_C|SetText_Headline (Variables|Default|GetW_NPC1_ref) "Gatekeeper")
      (Variables|/Game/MyContent/Widgets/W_NPC1.W_NPC1_C|SetText_Body (Variables|Default|GetW_NPC1_ref) (Utilities|String|MakeLiteralString "That statue was everyhing to me! 
If I ever see one of those conquerers again... I will smash them with my hammer!"))
      (if (Variables|/Game/MyContent/BluePrints/SM_Plains_Angel_Statue_01_Blueprint.SM_Plains_Angel_Statue_01_Blueprint_C|GetFoundSmallStatue (Variables|Dialog|GetBP_Ref_SmallStatue))
        (Variables|/Game/MyContent/Widgets/W_NPC1.W_NPC1_C|SetText_Body (Variables|Default|GetW_NPC1_ref) (Utilities|String|MakeLiteralString "My beloved statue! 
I can't believe you found it! 
I am forever in your debt, you are a true Hero!"))
        (bind _asthird_person_character (Utilities|Casting|CastToThirdPersonCharacter (Game|GetPlayerCharacter 0)))
        (Variables|/Game/ThirdPersonBP/Blueprints/ThirdPersonCharacter.ThirdPersonCharacter_C|SetbQuestComplete _asthird_person_character true))
      (else
        (Variables|Default|SetbFirstTalkEnded true)))))

(fn ConstructionScript
  (Components|Box|SetBoxExtent (Variables|Default|GetTriggerZone) (Variables|Construction|GetTriggerBoxSize) true))