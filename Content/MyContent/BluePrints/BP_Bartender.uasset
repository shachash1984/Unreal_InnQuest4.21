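; BP_Bartender is an interactable bartender actor that opens a W_Bartender UI when the player talks to it.
; Its BarTriggerZone enables the actor's input when the player character enters and disables it when they leave.
; Pressing Action creates the widget on first use and reuses the cached reference afterwards, adds it to the viewport and switches the controller to UI-only input.
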(event OnComponentEndOverlap(BarTriggerZone)
  (params (OverlappedComponent :type Primitive%20Component%20Object%20Reference) (OtherActor :type Actor%20Object%20Reference) (OtherComp :type Primitive%20Component%20Object%20Reference) (OtherBodyIndex :type Integer))
  ;[1 1 1] GateKeeper Triggerzone
  (if (== OtherActor (Game|GetPlayerCharacter 0))
    (Input|DisableInput (Game|GetPlayerController 0))))

(event OnComponentBeginOverlap(BarTriggerZone)
  (params (OverlappedComponent :type Primitive%20Component%20Object%20Reference) (OtherActor :type Actor%20Object%20Reference) (OtherComp :type Primitive%20Component%20Object%20Reference) (OtherBodyIndex :type Integer) (bFromSweep :type Boolean) (SweepResult :type Hit%20Result%20Structure%20%28by%20ref%29))
  ;[1 1 1] GateKeeper Triggerzone
  (if (== OtherActor (Game|GetPlayerCharacter 0))
    (Input|EnableInput (Game|GetPlayerController 0))))

(event EventBeginPlay)

(event Collision|EventActorBeginOverlap
  (params (OtherActor :type Actor%20Object%20Reference)))

(event EventTick
  (params (DeltaSeconds :type Float%20%28single-precision%29)))

(event Input|ActionEvents|InputActionAction
  (params (Key :type Key%20Structure :default "AnyKey"))
  (bind _returnvalue (Game|GetPlayerController 0))
  ;[1 1 1] Talking to the GateKeeper
  (:Pressed
    (Utilities|IsValid (Variables|Default|GetW_Bartender_ref)
      (:Is%20Valid
        _)
      (:Is%20Not%20Valid
        (bind _returnvalue_2 (UserInterface|CreateWidget "/Game/MyContent/Widgets/W_Bartender.W_Bartender_C" _returnvalue))
        (bind _output_get (Variables|Default|SetW_Bartender_ref _returnvalue_2))))
    (UserInterface|Viewport|AddtoViewport _output_get 0)
    (Input|SetInputModeUIOnly _returnvalue 0 "DoNotLock")))

(fn ConstructionScript)